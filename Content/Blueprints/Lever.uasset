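; Interactable lever that sends turn-on or turn-off messages to the other actors it controls.
; A collider enables input and prints an interact prompt while the FirstPersonCharacter overlaps it, and disables input on exit.
; Pressing Interact sends the message and plays or reverses the Move timeline, which drives the lever's pitch.
; The On state flips only when the timeline finishes.
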(event OnComponentBeginOverlap(collider)
  (params (OverlappedComponent :type Primitive%20Component%20Object%20Reference) (OtherActor :type Actor%20Object%20Reference) (OtherComp :type Primitive%20Component%20Object%20Reference) (OtherBodyIndex :type Integer) (bFromSweep :type Boolean) (SweepResult :type Hit%20Result%20Structure%20%28by%20ref%29))
  (Utilities|Casting|CastToFirstPersonCharacter OtherActor)
  (Input|EnableInput (Game|GetPlayerController 0))
  (Development|PrintString "Press 'e' to interact"))

(event OnComponentEndOverlap(collider)
  (params (OverlappedComponent :type Primitive%20Component%20Object%20Reference) (OtherActor :type Actor%20Object%20Reference) (OtherComp :type Primitive%20Component%20Object%20Reference) (OtherBodyIndex :type Integer))
  (Utilities|Casting|CastToFirstPersonCharacter OtherActor)
  (Input|DisableInput (Game|GetPlayerController 0)))

(event Input|ActionEvents|InputActionInteract
  (params (Key :type Key%20Structure :default "None"))
  (bind _other_actors_controlled_by_this_actor (Variables|Default|Getother%20actors%20controlled%20by%20this%20actor))
  (:Pressed
    (if (not (Variables|Default|Geton))
      (Class|ToggleableObject|Turnon(Message) _other_actors_controlled_by_this_actor)
      (bind _move (Timeline|Move Play)
        (:Update
          (Transformation|SetRelativeLocationAndRotation (Variables|Default|Getlever) (Math|Vector|MakeVector 0.0 0.0 0.0) (Math|Rotator|MakeRotator 0.0 _move 0.0) false false))
        (:Finished
          (if (Variables|Default|Geton)
            (Variables|Default|Seton false)
            (else
              (Variables|Default|Seton true)))))
      (else
        (Class|ToggleableObject|TurnOff(Message) _other_actors_controlled_by_this_actor)
        (Timeline|Move Reverse)))))

(fn ConstructionScript)