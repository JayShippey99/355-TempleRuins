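; LED Blueprint that cycles its color through red, green and blue each time its Trigger event fires.
; The construction script creates a dynamic material instance on the Thing component and applies the color for the current state.
; Trigger advances the state enum with a Select node, then UpdateColor maps it to the material's Color parameter.
; An equivalent switch-based version of the state change remains in the graph, unconnected.
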(event EventTrigger
  ;[1 1 1] change state w select
  (Variables|Default|SetCurrentState (Utilities|Select :Index (Variables|Default|GetCurrentState) :NewEnumerator0 "NewEnumerator1" :NewEnumerator1 "NewEnumerator2" :NewEnumerator2 "NewEnumerator0"))
  (CallFunction|UpdateColor))

(fn ConstructionScript
  (bind _returnvalue (Rendering|Material|CreateDynamicMaterialInstance (Variables|Default|Getthing) 0 "/Game/Blueprints/LED/LEDMat.LEDMat" "None" :!class /Script/Engine.PrimitiveComponent))
  (Variables|Default|SetLEDMaterial _returnvalue)
  (CallFunction|UpdateColor))

(fn UpdateColor
  ;[1 1 1] update the material
  (Rendering|Material|SetVectorParameterValue (Variables|Default|GetLEDMaterial) "Color" (Utilities|Select :Index (Variables|Default|GetCurrentState) :NewEnumerator0 "(R=1.000000,G=0.000000,B=0.000000,A=1.000000)" :NewEnumerator1 "(R=0.000000,G=1.000000,B=0.000000,A=1.000000)" :NewEnumerator2 "(R=0.000000,G=0.000000,B=1.000000,A=1.000000)") :!class /Script/Engine.MaterialInstanceDynamic))