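; Elevator actor that raises a Mover component up to MaxHeight when the player presses Interact inside its trigger.
; An Elevate timeline drives the Mover's relative Z, with play rate set on BeginPlay from MaxHeight divided by Speed.
; Collider overlap with the FirstPersonCharacter enables input on the actor, so Interact only works inside it.
; Leaving the Collider disables input and reverses the timeline.
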(event OnComponentBeginOverlap(Collider)
  (params (OverlappedComponent :type Primitive%20Component%20Object%20Reference) (OtherActor :type Actor%20Object%20Reference) (OtherComp :type Primitive%20Component%20Object%20Reference) (OtherBodyIndex :type Integer) (bFromSweep :type Boolean) (SweepResult :type Hit%20Result%20Structure%20%28by%20ref%29))
  ;[1 1 1] OHHH this only allows player input when colliding
  (Utilities|Casting|CastToFirstPersonCharacter OtherActor)
  (Input|EnableInput (Game|GetPlayerController 0)))

(event OnComponentEndOverlap(Collider)
  (params (OverlappedComponent :type Primitive%20Component%20Object%20Reference) (OtherActor :type Actor%20Object%20Reference) (OtherComp :type Primitive%20Component%20Object%20Reference) (OtherBodyIndex :type Integer))
  ;[1 1 1] OHHH this only allows player input when colliding
  (Utilities|Casting|CastToFirstPersonCharacter OtherActor)
  (Input|DisableInput (Game|GetPlayerController 0))
  (bind _percent (Timeline|Elevate Reverse)
    (:Update
      (Transformation|SetRelativeLocation (Variables|Default|GetMover) (Math|Vector|MakeVector 0.0 0.0 (* _percent (Variables|Default|GetMax%20Height))) false false))))

(event EventBeginPlay
  (Components|Timeline|SetPlayRate (Variables|Default|GetElevate) (/ (Variables|Default|GetMax%20Height) (Variables|Default|GetSpeed))))

(event Input|ActionEvents|InputActionInteract
  (params (Key :type Key%20Structure :default "None"))
  (:Pressed
    (bind _percent (Timeline|Elevate Play)
      (:Update
        (Transformation|SetRelativeLocation (Variables|Default|GetMover) (Math|Vector|MakeVector 0.0 0.0 (* _percent (Variables|Default|GetMax%20Height))) false false)))))

(fn ConstructionScript)