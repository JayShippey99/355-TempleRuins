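; Rideable minecart Blueprint on a spline track: the player possesses it on interact, looks around, and exits as a newly spawned FirstPersonCharacter at the camera.
; The construction script lays fixed-length spline mesh pieces along the track.
; Tick adjusts clamped velocity from forward/backward flags, then places Mover at PositionOnSpline.
; The step advancing PositionOnSpline by Velocity and the flag resets are disconnected, so the cart never travels.
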(event EventPlayerWantstoInteract
  (params (Player :type First%20Person%20Character%20Object%20Reference))
  ;[1 1 1] get in minecart
  (Pawn|Possess (Pawn|GetController Player) self)
  (Actor|DestroyActor Player))

(event EventTick
  (params (DeltaSeconds :type Float%20%28single-precision%29))
  (CallFunction|Accelerate DeltaSeconds)
  (CallFunction|PositionCart))

(event Input|ActionEvents|InputActionInteract
  (params (Key :type Key%20Structure :default "None"))
  (bind _camera (Variables|Default|GetCamera))
  (bind _returnvalue (Transformation|GetWorldTransform _camera))
  ;[1 1 1] somehthing
  (:Pressed
    (bind _returnvalue_2 (Game|SpawnActorfromClass "/Game/Blueprints/FirstPersonCharacter.FirstPersonCharacter_C" (Math|Transform|MakeTransform (.location _returnvalue) (Math|Rotator|MakeRotator 0.0 0.0 (.yaw (.rotation _returnvalue))) "1,1,1") "Undefined" (Components|GetOwner) 0))
    (Transformation|SetWorldRotation (Variables|/Game/Blueprints/FirstPersonCharacter.FirstPersonCharacter_C|GetFirstPersonCamera _returnvalue_2) (Math|Rotator|MakeRotator 0.0 (.pitch (.rotation _returnvalue)) (.yaw (.rotation _returnvalue))) false false)
    (Pawn|Possess (Pawn|GetController) _returnvalue_2)))

(event Input|ActionEvents|InputActionminecartforward
  (params (Key :type Key%20Structure :default "None")))

(event Input|ActionEvents|InputActionminecartbackward
  (params (Key :type Key%20Structure :default "None")))

(event Input|AxisEvents|InputAxisTurn
  (params (AxisValue :type Float%20%28single-precision%29))
  ;[1 1 1] Mouse look
  (Pawn|Input|AddControllerYawInput AxisValue))

(event Input|AxisEvents|InputAxisLookUp
  (params (AxisValue :type Float%20%28single-precision%29))
  ;[1 1 1] Mouse look
  (Pawn|Input|AddControllerPitchInput AxisValue))

(event Input|AxisEvents|InputAxisTurnRate
  (params (AxisValue :type Float%20%28single-precision%29))
  ;[1 1 1] stick look
  (Pawn|Input|AddControllerYawInput (* AxisValue 45.0 (Utilities|Time|GetWorldDeltaSeconds))))

(event Input|AxisEvents|InputAxisLookUpRate
  (params (AxisValue :type Float%20%28single-precision%29))
  ;[1 1 1] stick look
  (Pawn|Input|AddControllerPitchInput (* AxisValue 45.0 (Utilities|Time|GetWorldDeltaSeconds))))

(fn ConstructionScript
  (bind _spline (Variables|Default|GetSpline))
  (bind _spline_2 (Variables|Default|GetSpline))
  (CallFunction|PositionCart)
  (for _index (range 0 (- (Math|Float|Truncate (/ (Spline|GetSplineLength (Variables|Default|GetSpline)) (Variables|Default|Getlength%20of%20piece))) 1))
    (bind _returnvalue (AddComponent|AddSplineMeshComponent false))
    (SplineMesh|SetStartandEnd _returnvalue (Spline|GetLocationatDistanceAlongSpline _spline_2 (* _index (Variables|Default|Getlength%20of%20piece)) "Local") (Math|Vector|ClampVectorSize (Spline|GetTangentatDistanceAlongSpline _spline_2 (* _index (Variables|Default|Getlength%20of%20piece)) "Local") 0.0 (Variables|Default|Getlength%20of%20piece)) (Spline|GetLocationatDistanceAlongSpline _spline (* (+ _index 1) (Variables|Default|Getlength%20of%20piece)) "Local") (Math|Vector|ClampVectorSize (Spline|GetTangentatDistanceAlongSpline _spline (* (+ _index 1) (Variables|Default|Getlength%20of%20piece)) "Local") 0.0 (Variables|Default|Getlength%20of%20piece)) true :!class /Script/Engine.SplineMeshComponent)))

(fn PositionCart
  (bind _position_on_spline (Variables|Default|Getposition%20on%20spline))
  (bind _spline (Variables|Default|GetSpline))
  (Transformation|SetRelativeLocationAndRotation (Variables|Default|GetMover) (Spline|GetLocationatDistanceAlongSpline _spline _position_on_spline "Local") (Spline|GetRotationatDistanceAlongSpline _spline _position_on_spline "Local") false false))

(fn Accelerate
  (params (Delta%20Time :type Float%20%28single-precision%29))
  (bind _maxvelocity (Variables|Default|GetmaxVelocity))
  (if (Variables|Default|Getplayer%20wants%20to%20move%20forward)
    (LocalVariables|SetDirection 1.0)
    (Variables|Default|Setvelocity (Math|Float|Clamp(Float) (+ (Variables|Default|Getvelocity) (* (LocalVariables|GetDirection) Delta%20Time (Variables|Default|GetaccelerationMultiplier))) (* _maxvelocity -1.0) _maxvelocity) :!label _label)
    (elif (Variables|Default|Getplayer%20wants%20to%20move%20backward)
      (LocalVariables|SetDirection (- (LocalVariables|GetDirection) 1.0))
      (goto _label))))