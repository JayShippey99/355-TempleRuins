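; Drivable UFO pawn that a first-person player can board and leave.
; Boarding possesses the UFO and destroys the character; Interact spawns a new character at the UFO camera, matches its view and possesses it.
; Mouse and stick axes steer the view, while move axes push the Bubble component with forces along the actor's forward and right vectors.
; Unconnected leftover nodes hint at an unfinished tilt feature.
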(event EventPlayerWantstoInteract
  (params (Player :type First%20Person%20Character%20Object%20Reference))
  ;[1 1 1] get in UFo
  (Pawn|Possess (Pawn|GetController Player) self)
  (Actor|DestroyActor Player))

(event Input|ActionEvents|InputActionInteract
  (params (Key :type Key%20Structure :default "None"))
  (bind _camera (Variables|Default|GetCamera))
  (bind _returnvalue (Transformation|GetWorldTransform _camera))
  ;[1 1 1] somehthing
  (:Pressed
    (bind _returnvalue_2 (Game|SpawnActorfromClass "/Game/Blueprints/FirstPersonCharacter.FirstPersonCharacter_C" (Math|Transform|MakeTransform (.location _returnvalue) (Math|Rotator|MakeRotator 0.0 0.0 (.yaw (.rotation _returnvalue))) "1,1,1") "Undefined" (Components|GetOwner) 0))
    (Transformation|SetWorldRotation (Variables|/Game/Blueprints/FirstPersonCharacter.FirstPersonCharacter_C|GetFirstPersonCamera _returnvalue_2) (Math|Rotator|MakeRotator 0.0 (.pitch (.rotation _returnvalue)) (.yaw (.rotation _returnvalue))) false false)
    (Pawn|Possess (Pawn|GetController) _returnvalue_2)))

(event Input|AxisEvents|InputAxisMoveForward
  (params (AxisValue :type Float%20%28single-precision%29))
  ;[1 1 1] move
  (Physics|AddForce (Variables|Default|Getbubble) (* (* (Transformation|GetActorForwardVector) AxisValue) (Variables|Default|GetVeclocity)) "None" false))

(event Input|AxisEvents|InputAxisTurn
  (params (AxisValue :type Float%20%28single-precision%29))
  ;[1 1 1] Mouse look
  (Pawn|Input|AddControllerYawInput AxisValue))

(event Input|AxisEvents|InputAxisLookUp
  (params (AxisValue :type Float%20%28single-precision%29))
  ;[1 1 1] Mouse look
  (Pawn|Input|AddControllerPitchInput AxisValue))

(event Input|AxisEvents|InputAxisMoveRight
  (params (AxisValue :type Float%20%28single-precision%29))
  ;[1 1 1] move
  (Physics|AddForce (Variables|Default|Getbubble) (* (* (Transformation|GetActorRightVector) AxisValue) (Variables|Default|GetVeclocity)) "None" false))

(event Input|AxisEvents|InputAxisTurnRate
  (params (AxisValue :type Float%20%28single-precision%29))
  ;[1 1 1] stick look
  (Pawn|Input|AddControllerYawInput (* AxisValue 45.0 (Utilities|Time|GetWorldDeltaSeconds))))

(event Input|AxisEvents|InputAxisLookUpRate
  (params (AxisValue :type Float%20%28single-precision%29))
  ;[1 1 1] stick look
  (Pawn|Input|AddControllerPitchInput (* AxisValue 45.0 (Utilities|Time|GetWorldDeltaSeconds))))

(fn ConstructionScript)